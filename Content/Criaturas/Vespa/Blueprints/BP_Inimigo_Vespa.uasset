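; Wasp enemy that wanders the map, chases seen pawns and feeds the player's wasp kill quest.
; Looping AI MoveTo roams random reachable points; PawnSensing redirects it to the pawn, playing a random attack montage on arrival.
; Tick shows a player-facing health bar widget when the player is near.
; AnyDamage plays a hit montage, blocking attacks, then at low health plays death, updates the active quest's count and HUD, and destroys the actor.
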(event `Andar Pelo Mapa`
  ;[1 1 1] Andar pelo mapa de modo aleatorio
  (`|AIMoveTo` self (`NavigationSystemV1.K2_GetRandomReachablePointInRadius` (`self.K2_GetActorLocation`) 3000.0 null null) null
    (:`OnSuccess`
      _)
    (:`OnFail`
      _))
  (`KismetSystemLibrary.Delay` 5.0)
  (`self.Andar Pelo Mapa`))

(event `self.ReceiveBeginPlay`
  ;[1 1 1] Andar pelo mapa de modo aleatorio
  (`self.Andar Pelo Mapa`))

(event `self.PawnSensing.OnSeePawn`
  (params (Pawn :type "Pawn Object Reference"))
  ;[1 1 1] Seguir o Player que ver
  (`|AIMoveTo` self (0.0 0.0 0.0) Pawn 10.0
    (:`OnSuccess`
      ;[1 1 1] Bater quando chegar perto
      (if (`self.Pode Levar Dano?`)
        (`CharacterMovementComponent.DisableMovement` (`self.CharacterMovement`))
        (`|PlayMontage` (`self.Mesh`) (`KismetArrayLibrary.Array_Random` (`self.Montage Ataque Vespa`)) 1.0 0.0 "None" false
          (:`then`
            (`GameplayStatics.PlaySound2D` "/Game/Criaturas/Vespa/Audio/Idle_Vespa.Idle_Vespa" 1.0 1.0 0.0 null null))
          (:`OnCompleted`
            (`CharacterMovementComponent.SetMovementMode` (`self.CharacterMovement`) "MOVE_Walking" 0 :!label _label)
            (`self.Andar Pelo Mapa`))
          (:`OnInterrupted`
            (goto _label)))))))

(event `self.ReceiveTick`
  (params (DeltaSeconds :type "Float (single-precision)"))
  (bind _barra_de_vida_vespa (`self.Barra de Vida Vespa`))
  (bind _barra_de_vida_vespa_2 (`self.Barra de Vida Vespa`))
  ;[1 1 1] Barra de vida do inimigo
  (if (< (`KismetMathLibrary.VSize` (- (`self.K2_GetActorLocation` (`GameplayStatics.GetPlayerCharacter` 0)) (`self.K2_GetActorLocation`))) 2000.0)
    (`SceneComponent.SetVisibility` _barra_de_vida_vespa true false)
    (`SceneComponent.K2_SetWorldRotation` _barra_de_vida_vespa_2 (`KismetMathLibrary.FindLookAtRotation` (`self.K2_GetActorLocation`) (`self.K2_GetActorLocation` (`GameplayStatics.GetPlayerCharacter` 0))) false false)
    (bind _aswb_barra_de_vida_inimigo_vespa (cast `/Game/Criaturas/Vespa/Blueprints/WB_Barra_de_Vida_Inimigo_Vespa` (`WidgetComponent.GetWidget` _barra_de_vida_vespa_2)))
    (`ProgressBar.SetPercent` (`/Game/Criaturas/Vespa/Blueprints/WB_Barra_de_Vida_Inimigo_Vespa.BarradevidadoinimigoVespa` _aswb_barra_de_vida_inimigo_vespa) (/ (`self.Vida Atual`) 50.0))
    (else
      (`SceneComponent.SetVisibility` _barra_de_vida_vespa false false))))

(event `self.ReceiveAnyDamage`
  (params (Damage :type "Float (single-precision)") (DamageType :type "DamageType Object Reference") (InstigatedBy :type "Controller Object Reference") (DamageCauser :type "Actor Object Reference"))
  ;[1 1 1] Inimigo leva dano e efetua a animação de dano, além de morrer se a barra de vida for menor ou igual a 0
  (set `self.Pode Levar Dano?` false)
  (`|PlayMontage` (`self.Mesh`) "/Game/Criaturas/Vespa/Animação/ANM_Levando_Dano_Vespa.ANM_Levando_Dano_Vespa" 1.7
    (:`then`
      (bind _output_get (set `self.Vida Atual` (- (`self.Vida Atual`) Damage))))
    (:`OnCompleted`
      (if (> _output_get 1.0)
        (set `self.Pode Levar Dano?` true)
        (else
          (`CharacterMovementComponent.DisableMovement` (`self.CharacterMovement`))
          (`|PlayMontage` (`self.Mesh`) "/Game/Criaturas/Vespa/Animação/ANM_Morrendo_Inimigo_Vespa.ANM_Morrendo_Inimigo_Vespa" 0.5
            (:`then`
              (bind _asbp_third_person_character (cast `/Game/ThirdPerson/Blueprints/BP_ThirdPersonCharacter` (`GameplayStatics.GetPlayerCharacter` 0)))
              (if (`/Game/ThirdPerson/Blueprints/BP_ThirdPersonCharacter.QuestVespasAceita` _asbp_third_person_character)
                (if (not (`/Game/ThirdPerson/Blueprints/BP_ThirdPersonCharacter.QuestVespasConcluida` _asbp_third_person_character))
                  (set `/Game/ThirdPerson/Blueprints/BP_ThirdPersonCharacter.VespasMortas` (+ (`/Game/ThirdPerson/Blueprints/BP_ThirdPersonCharacter.VespasMortas` _asbp_third_person_character) 1) _asbp_third_person_character)
                  (`/Game/Programação_Geral/Missoes/NPC_Vespa/WB_Quest_Vespa.AtualizarProgressoVespas` (`/Game/ThirdPerson/Blueprints/BP_ThirdPersonCharacter.QuestVespaHUDRef` _asbp_third_person_character) (`/Game/ThirdPerson/Blueprints/BP_ThirdPersonCharacter.VespasMortas` _asbp_third_person_character)))))
            (:`OnCompleted`
              (`self.K2_DestroyActor`))))))))

(fn `Bear dead`)

(fn `UserConstructionScript`)