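; Quest-giver NPC for the bear quest, ending with the victory screen.
; Sphere overlap toggles input and a prompt turned toward the player; E steps through indexed intro and final dialogue using quest flags on the player.
; Accepting shows the quest HUD and hides linked structures; their re-show loop is unconnected.
; After the kill, interactions mark completion, play Niagara, then run closing dialogue and a timed transition.
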(event `self.ReceiveBeginPlay`
  ; Estruturas começam invisivéis no começo do jogo
)

(event `self.Sphere.OnComponentBeginOverlap`
  (params (OverlappedComponent :type "PrimitiveComponent Object Reference") (OtherActor :type "Actor Object Reference") (OtherComp :type "PrimitiveComponent Object Reference") (OtherBodyIndex :type Integer) (bFromSweep :type Boolean) (SweepResult :type "HitResult Structure (by ref)"))
  ; Colidir com o NPC para aparecer a Interação
  (bind _asbp_third_person_character (cast `/Game/ThirdPerson/Blueprints/BP_ThirdPersonCharacter` OtherActor))
  (bind _output_get (set `self.PlayerRef` _asbp_third_person_character))
  (`self.EnableInput` (`GameplayStatics.GetPlayerController` 0))
  (set `/Game/ThirdPerson/Blueprints/BP_ThirdPersonCharacter.ColidindoQuestVespa?` true _output_get)
  (`SceneComponent.SetHiddenInGame` (`self.Texto`) false false)
  (`SceneComponent.K2_SetWorldRotation` (`self.Texto`) (`KismetMathLibrary.FindLookAtRotation` (`self.K2_GetActorLocation`) (`self.K2_GetActorLocation` (`GameplayStatics.GetPlayerCharacter` 0))) false false))

(event `self.Sphere.OnComponentEndOverlap`
  (params (OverlappedComponent :type "PrimitiveComponent Object Reference") (OtherActor :type "Actor Object Reference") (OtherComp :type "PrimitiveComponent Object Reference") (OtherBodyIndex :type Integer))
  ; Colidir com o NPC para aparecer a Interação
  (bind _asbp_third_person_character (cast `/Game/ThirdPerson/Blueprints/BP_ThirdPersonCharacter` OtherActor))
  (bind _output_get (set `self.PlayerRef` _asbp_third_person_character))
  (`self.DisableInput` (`GameplayStatics.GetPlayerController` 0))
  (set `/Game/ThirdPerson/Blueprints/BP_ThirdPersonCharacter.ColidindoQuestVespa?` false _output_get)
  (`SceneComponent.SetHiddenInGame` (`self.Texto`) true false)
  (`self.DisableInput` (`GameplayStatics.GetPlayerController` 0)))

(event `Key|E`
  (params (Key :type "Key Structure"))
  (bind _playerref (`self.PlayerRef`))
  (bind _playerref_2 (`self.PlayerRef`))
  (bind _playerref_3 (`self.PlayerRef`))
  (bind _playerref_4 (`self.PlayerRef`))
  (bind _dialogonpcref (`/Game/ThirdPerson/Blueprints/BP_ThirdPersonCharacter.DialogoNPCRef` (`self.PlayerRef`)))
  (bind _dialogonpcref_2 (`/Game/ThirdPerson/Blueprints/BP_ThirdPersonCharacter.DialogoNPCRef` (`self.PlayerRef`)))
  ; interagir com o NPC (E)
  (:`Pressed`
    (`/Engine/EditorBlueprintResources/StandardMacros.IsValid` _playerref_3
      (:`Is Valid`
        (if (`/Game/ThirdPerson/Blueprints/BP_ThirdPersonCharacter.QuestUrsoConcluida` _playerref_3)
          (if (`/Game/ThirdPerson/Blueprints/BP_ThirdPersonCharacter.EfeitoQuestUrsoJaTocou` (`self.PlayerRef`))
            (switch `int` (`KismetMathLibrary.Conv_Int64ToInt` (`self.FinalQuestIndex`))
              (:`0`
                (`/Game/Programação_Geral/Missoes/WB_Dialogo_NPC.MostrarDialogoUrso` _dialogonpcref_2 "Você voltou... então conseguiu enfrentar o urso da clareira. Poucos teriam coragem para encarar uma criatura tão forte.")
                (set `self.FinalQuestIndex` 1))
              (:`1`
                (`/Game/Programação_Geral/Missoes/WB_Dialogo_NPC.MostrarDialogoUrso` _dialogonpcref_2 "Com ele fora do caminho, a mina ficará muito mais segura. A vila deve lembrar do que você fez hoje. Obrigado.")
                (set `self.FinalQuestIndex` 2))
              (:`2`
                (`/Game/Programação_Geral/Missoes/WB_Dialogo_NPC.EsconderDialogoUrso` _dialogonpcref_2)
                (`/Game/Programação_Geral/Missoes/Wb_Quest.EsconderMissãoUrso` (`/Game/ThirdPerson/Blueprints/BP_ThirdPersonCharacter.QuestHUDRef` (`self.PlayerRef`)))
                (if (not (`/Game/ThirdPerson/Blueprints/BP_ThirdPersonCharacter.EfeitoTransiçãoJáPassou` _playerref_2))
                  (`Widget.SetVisibility` (`/Game/ThirdPerson/Blueprints/BP_ThirdPersonCharacter.TransicaoQuestRef` _playerref_2) "Visible")
                  (`KismetSystemLibrary.Delay` 0.5)
                  (`KismetSystemLibrary.Delay` 0.5)
                  (`Widget.SetVisibility` (`/Game/ThirdPerson/Blueprints/BP_ThirdPersonCharacter.TransicaoQuestRef` _playerref_4) "Hidden")
                  (set `/Game/ThirdPerson/Blueprints/BP_ThirdPersonCharacter.EfeitoTransiçãoJáPassou` true _playerref_4)
                  (set `self.FinalQuestIndex` 3)))
              (:`3`
                (`Widget.SetVisibility` (`/Game/ThirdPerson/Blueprints/BP_ThirdPersonCharacter.TelaVitoriaRef` _playerref_2) "Visible")
                (set `PlayerController.bShowMouseCursor` true (`PlayerState.GetPlayerController` (`Pawn.PlayerState` _playerref_2)))))
            (else
              (`ActorComponent.SetActive` (`self.Niagara`) true true)
              (`KismetSystemLibrary.Delay` 1.0)
              (set `/Game/ThirdPerson/Blueprints/BP_ThirdPersonCharacter.EfeitoQuestUrsoJaTocou` true (`self.PlayerRef`))))
          (elif (`/Game/ThirdPerson/Blueprints/BP_ThirdPersonCharacter.QuestUrsoAceita` _playerref_3)
            (if (>= (`/Game/ThirdPerson/Blueprints/BP_ThirdPersonCharacter.UrsoMorto` (`self.PlayerRef`)) 1)
              (set `/Game/ThirdPerson/Blueprints/BP_ThirdPersonCharacter.QuestUrsoConcluida` true (`self.PlayerRef`)))
            (else
              (switch `int` (`KismetMathLibrary.Conv_Int64ToInt` (`self.IntroQuestIndex`))
                (:`0`
                  (`/Game/Programação_Geral/Missoes/WB_Dialogo_NPC.MostrarDialogoUrso` _dialogonpcref "A estrada da mina voltou a respirar, mas ainda há um perigo rondando por perto.")
                  (set `self.IntroQuestIndex` 1))
                (:`1`
                  (`/Game/Programação_Geral/Missoes/WB_Dialogo_NPC.MostrarDialogoUrso` _dialogonpcref "Na clareira próxima à mina, um urso enorme tomou conta do lugar. Ele é forte... forte demais para qualquer morador enfrentar.")
                  (set `self.IntroQuestIndex` 2))
                (:`2`
                  (`/Game/Programação_Geral/Missoes/WB_Dialogo_NPC.MostrarDialogoUrso` _dialogonpcref "Ninguém consegue passar por ali sem correr risco. Se ele continuar naquela clareira, a mina nunca será realmente segura.")
                  (set `self.IntroQuestIndex` 3))
                (:`3`
                  (`/Game/Programação_Geral/Missoes/WB_Dialogo_NPC.MostrarDialogoUrso` _dialogonpcref "Se tiver coragem, elimine o urso da clareira perto da mina e volte para falar comigo. Mas vá preparado... ele não cairá fácil.")
                  (set `self.IntroQuestIndex` 4))
                (:`4`
                  (`/Game/Programação_Geral/Missoes/WB_Dialogo_NPC.EsconderDialogoUrso` _dialogonpcref)
                  (set `/Game/ThirdPerson/Blueprints/BP_ThirdPersonCharacter.QuestUrsoAceita` true _playerref)
                  (set `/Game/ThirdPerson/Blueprints/BP_ThirdPersonCharacter.EfeitoTransiçãoJáPassou` false _playerref)
                  (set `/Game/ThirdPerson/Blueprints/BP_ThirdPersonCharacter.UrsoMorto` 0 _playerref)
                  (`/Game/Programação_Geral/Missoes/Wb_Quest.MostrarQuestUrso` (`/Game/ThirdPerson/Blueprints/BP_ThirdPersonCharacter.QuestHUDRef` _playerref))
                  (for _array_element (`self.EstruturasParaAparecerUrso`)
                    (`self.SetActorHiddenInGame` _array_element true)
                    (`self.SetActorEnableCollision` _array_element false)))))))))))

(fn `UserConstructionScript`)