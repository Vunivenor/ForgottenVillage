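; Anim notify state for the bear enemy's attack (Urso) that deals melee damage during its animation window.
; Each tick sphere-traces on Visibility between two right-hand sockets, with debug draw, and applies fixed damage to the hit actor.
; Begin and end both clear BP_Inimigo_Urso's JáAcertou ("already hit") flag, but the tick never reads or sets it, so damage can repeat every tick.
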(fn `Received_NotifyBegin`
  (params (MeshComp :type "SkeletalMeshComponent Object Reference") (Animation :type "AnimSequenceBase Object Reference") (TotalDuration :type "Float (single-precision)") (EventReference :type "AnimNotifyEventReference Structure (by ref)"))
  (returns (ReturnValue :type Boolean))
  (bind _asbp_inimigo_urso (cast `/Game/Criaturas/Urso/Blueprints/BP_Inimigo_Urso` (`ActorComponent.GetOwner` MeshComp)))
  (set `/Game/Criaturas/Urso/Blueprints/BP_Inimigo_Urso.Já Acertou?` false _asbp_inimigo_urso)
  (return false))

(fn `Received_NotifyEnd`
  (params (MeshComp :type "SkeletalMeshComponent Object Reference") (Animation :type "AnimSequenceBase Object Reference") (EventReference :type "AnimNotifyEventReference Structure (by ref)"))
  (returns (ReturnValue :type Boolean))
  (bind _asbp_inimigo_urso (cast `/Game/Criaturas/Urso/Blueprints/BP_Inimigo_Urso` (`ActorComponent.GetOwner` MeshComp)))
  (set `/Game/Criaturas/Urso/Blueprints/BP_Inimigo_Urso.Já Acertou?` false _asbp_inimigo_urso)
  (return false))

(fn `Received_NotifyTick`
  (params (MeshComp :type "SkeletalMeshComponent Object Reference") (Animation :type "AnimSequenceBase Object Reference") (FrameDeltaTime :type "Float (single-precision)") (EventReference :type "AnimNotifyEventReference Structure (by ref)"))
  (returns (ReturnValue :type Boolean))
  (bind _outhit (`KismetSystemLibrary.SphereTraceSingle` :`WorldContextObject` MeshComp :`Start` (`SceneComponent.GetSocketLocation` MeshComp "hand_rSoquete_Urso") :`End` (`SceneComponent.GetSocketLocation` MeshComp "hand_rSoquete_Urso_0") :`Radius` 15.0 :`TraceChannel` "TraceTypeQuery1" :`DrawDebugType` "ForDuration"))
  (`GameplayStatics.ApplyDamage` (`.HitActor` (`GameplayStatics.BreakHitResult` _outhit)) 5.0)
  (return false))