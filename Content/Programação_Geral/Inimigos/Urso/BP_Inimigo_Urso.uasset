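; Bear enemy that roams to random reachable points, chases pawns it senses and plays an attack animation on arrival, with no damage wired.
; A retriggerable delay resumes wandering after the last sighting.
; Tick shows a player-facing health bar widget within range and updates its percent.
; Damage plays a hit montage, then subtracts health; death destroys the actor, followed by widget removal and a delayed win-widget creation never added to viewport.
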(event `Andar Pelo Mapa`
  ;[1 1 1] Andar pelo mapa de modo aleatorio
  (`|AIMoveTo` self (`NavigationSystemV1.K2_GetRandomReachablePointInRadius` (`self.K2_GetActorLocation`) 3000.0 null null) null
    (:`OnSuccess`
      (`KismetSystemLibrary.Delay` 1.0)
      (`self.Andar Pelo Mapa`))))

(event `self.ReceiveBeginPlay`
  ;[1 1 1] Andar pelo mapa de modo aleatorio
  (`self.Andar Pelo Mapa`))

(event `self.PawnSensing.OnSeePawn`
  (params (Pawn :type "Pawn Object Reference"))
  ;[1 1 1] Seguir o Player que ver
  (`|ExecutionSequence`
    (:`then_0`
      (`|AIMoveTo` self (0.0 0.0 0.0) Pawn 10.0
        (:`OnSuccess`
          ;[1 1 1] Animação de atacar quando chega perto
          (`CharacterMovementComponent.DisableMovement` (`self.CharacterMovement`))
          (`SkeletalMeshComponent.PlayAnimation` (`self.Mesh`) "/Game/StylizedCreaturesBundle/Animations/Bear/A_Bear_Combat_Unarmed_Attack.A_Bear_Combat_Unarmed_Attack" false)
          (`|ExecutionSequence`
            (:`then_0`
              (`KismetSystemLibrary.Delay` 1.7)
              (`SkeletalMeshComponent.SetAnimationMode` (`self.Mesh`) "AnimationBlueprint" true)
              (`CharacterMovementComponent.SetMovementMode` (`self.CharacterMovement`) "MOVE_Walking" 0))))))
    (:`then_1`
      (`KismetSystemLibrary.RetriggerableDelay` 1.5)
      (`self.Andar Pelo Mapa`))))

(event `self.ReceiveTick`
  (params (DeltaSeconds :type "Float (single-precision)"))
  (bind _barra_de_vida (`self.Barra de vida`))
  (bind _barra_de_vida_2 (`self.Barra de vida`))
  ;[1 1 1] Barra de vida do inimigo
  (if (< (`KismetMathLibrary.VSize` (- (`self.K2_GetActorLocation` (`GameplayStatics.GetPlayerCharacter` 0)) (`self.K2_GetActorLocation`))) 2000.0)
    (`SceneComponent.SetVisibility` _barra_de_vida true false)
    (`SceneComponent.K2_SetWorldRotation` _barra_de_vida_2 (`KismetMathLibrary.FindLookAtRotation` (`self.K2_GetActorLocation`) (`self.K2_GetActorLocation` (`GameplayStatics.GetPlayerCharacter` 0))) false false)
    (bind _aswb_barra_de_vida_inimigo_urso (cast `/Game/Programação_Geral/Inimigos/Urso/WB_Barra_de_Vida_Inimigo_Urso` (`WidgetComponent.GetWidget` _barra_de_vida_2)))
    (`ProgressBar.SetPercent` (`/Game/Programação_Geral/Inimigos/Urso/WB_Barra_de_Vida_Inimigo_Urso.Barradevidadoinimigourso` _aswb_barra_de_vida_inimigo_urso) (/ (`self.Vida Atual`) 100.0))
    (else
      (`SceneComponent.SetVisibility` _barra_de_vida false false))))

(event `self.ReceiveAnyDamage`
  (params (Damage :type "Float (single-precision)") (DamageType :type "DamageType Object Reference") (InstigatedBy :type "Controller Object Reference") (DamageCauser :type "Actor Object Reference"))
  ;[1 0 0] Barra de Vida, com animação de morte e levando dano (O Urso não está tocando a animação de levar dano)
  (`CharacterMovementComponent.DisableMovement` (`self.CharacterMovement`))
  (`|PlayMontage` (`self.Mesh`) "/Game/Programação_Geral/Inimigos/Urso/ANM_Levando_Dano_Urso.ANM_Levando_Dano_Urso" 3.0
    (:`OnCompleted`
      (set `self.Levando dano?` false)
      (set `self.Vida Atual` (- (`self.Vida Atual`) Damage))
      (`SkeletalMeshComponent.SetAnimationMode` (`self.Mesh`) "AnimationBlueprint" true)
      (`CharacterMovementComponent.SetMovementMode` (`self.CharacterMovement`) "MOVE_Walking" 0)
      (if (<= (`self.Vida Atual`) 0.0)
        (`CharacterMovementComponent.DisableMovement` (`self.CharacterMovement`))
        (`SkeletalMeshComponent.PlayAnimation` (`self.Mesh`) "/Game/StylizedCreaturesBundle/Animations/Bear/A_Bear_Death.A_Bear_Death" false)
        (`KismetSystemLibrary.Delay` 5.0)
        (`self.K2_DestroyActor`)
        (`WidgetLayoutLibrary.RemoveAllWidgets`)
        (`KismetSystemLibrary.Delay` 5.0)
        (`|CreateWidget` "/Game/Missoes/WP_Win.WP_Win_C" (`GameplayStatics.GetPlayerController` 0))))))

(fn `Bear dead`)

(fn `UserConstructionScript`)