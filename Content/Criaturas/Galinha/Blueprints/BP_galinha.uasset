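; BP_galinha is a chicken creature that wanders the map, takes damage and dies, reusing snake (Cobra) sounds and death animation.
; From BeginPlay it loops AI moves to random reachable points, pausing briefly between them.
; AnyDamage plays a random hit montage and subtracts health; at 1 or below it stops movement, plays death, destroys itself and plays a Quest sound.
; PodeLevarDano toggles around hits but is never checked here.
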(event `Andar Pelo Mapa`
  ;[1 1 1] Andar pelo mapa de modo aleatorio
  (`|AIMoveTo` self (`NavigationSystemV1.K2_GetRandomReachablePointInRadius` (`self.K2_GetActorLocation`) 3000.0 null null) null
    (:`then`
      (`GameplayStatics.PlaySound2D` "/Game/Criaturas/Cobra/Audio/Idle_Cobra.Idle_Cobra" 1.0 1.0 0.0 null null))
    (:`OnSuccess`
      (`KismetSystemLibrary.Delay` 2.0 :!label _label)
      (`self.Andar Pelo Mapa`))
    (:`OnFail`
      (goto _label))))

(event `self.ReceiveBeginPlay`
  ;[1 1 1] Andar pelo mapa de modo aleatorio
  (`self.Andar Pelo Mapa`))

(event `self.ReceiveAnyDamage`
  (params (Damage :type "Float (single-precision)") (DamageType :type "DamageType Object Reference") (InstigatedBy :type "Controller Object Reference") (DamageCauser :type "Actor Object Reference"))
  ;[1 1 1] Inimigo leva dano e efetua a animação de dano, além de morrer se a barra de vida for menor ou igual a 0
  (set `self.Pode Levar Dano?` false)
  (`|PlayMontage` (`self.Mesh`) (`KismetArrayLibrary.Array_Random` (`self.Montage Dano`))
    (:`then`
      (bind _output_get (set `self.Vida Atual` (- (`self.Vida Atual`) Damage))))
    (:`OnCompleted`
      (if (> _output_get 1.0) :!label _label_2
        (set `self.Pode Levar Dano?` true)
        (else
          (`CharacterMovementComponent.DisableMovement` (`self.CharacterMovement`))
          (`|PlayMontage` (`self.Mesh`) "/Game/Criaturas/Cobra/Animações/ANM_Morte_Cobra.ANM_Morte_Cobra" 0.5
            (:`OnCompleted`
              (`self.K2_DestroyActor`)
              (`GameplayStatics.PlaySound2D` "/Game/Audio/Quest.Quest" 1.0 1.0 0.0 null null))))))
    (:`OnInterrupted`
      (goto _label_2))))

(fn `UserConstructionScript`)