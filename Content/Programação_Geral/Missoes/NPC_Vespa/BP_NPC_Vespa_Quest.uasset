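; Quest-giver NPC for the wasp quest, which asks the player to clear the mine road of venomous wasps.
; Sphere overlap toggles input and the prompt text; pressing E advances dialogue and quest stages using indices and flags on the player character.
; Three kills allow completion, followed by a Niagara effect and closing dialogue.
; Structures hidden at BeginPlay then appear with collision behind a transition widget.
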(event `self.ReceiveBeginPlay`
  ; Estruturas começam invisivéis no começo do jogo
  (for _array_element (`self.EstruturasParaAparecer`)
    (`self.SetActorHiddenInGame` _array_element true)
    (`self.SetActorEnableCollision` _array_element false)))

(event `self.Sphere.OnComponentBeginOverlap`
  (params (OverlappedComponent :type "PrimitiveComponent Object Reference") (OtherActor :type "Actor Object Reference") (OtherComp :type "PrimitiveComponent Object Reference") (OtherBodyIndex :type Integer) (bFromSweep :type Boolean) (SweepResult :type "HitResult Structure (by ref)"))
  ; Colidir com o NPC para aparecer a Interação
  (bind _asbp_third_person_character (cast `/Game/ThirdPerson/Blueprints/BP_ThirdPersonCharacter` OtherActor))
  (bind _output_get (set `self.PlayerRef` _asbp_third_person_character))
  (`self.EnableInput` (`GameplayStatics.GetPlayerController` 0))
  (set `/Game/ThirdPerson/Blueprints/BP_ThirdPersonCharacter.ColidindoQuestVespa?` true _output_get)
  (`SceneComponent.SetHiddenInGame` (`self.Texto`) false false)
  (`SceneComponent.K2_SetWorldRotation` (`self.Texto`) (`KismetMathLibrary.FindLookAtRotation` (`self.K2_GetActorLocation`) (`self.K2_GetActorLocation` (`GameplayStatics.GetPlayerCharacter` 0))) false false))

(event `self.Sphere.OnComponentEndOverlap`
  (params (OverlappedComponent :type "PrimitiveComponent Object Reference") (OtherActor :type "Actor Object Reference") (OtherComp :type "PrimitiveComponent Object Reference") (OtherBodyIndex :type Integer))
  ; Colidir com o NPC para aparecer a Interação
  (bind _asbp_third_person_character (cast `/Game/ThirdPerson/Blueprints/BP_ThirdPersonCharacter` OtherActor))
  (bind _output_get (set `self.PlayerRef` _asbp_third_person_character))
  (`self.DisableInput` (`GameplayStatics.GetPlayerController` 0))
  (set `/Game/ThirdPerson/Blueprints/BP_ThirdPersonCharacter.ColidindoQuestVespa?` false _output_get)
  (`SceneComponent.SetHiddenInGame` (`self.Texto`) true false)
  (`self.DisableInput` (`GameplayStatics.GetPlayerController` 0)))

(event `Key|E`
  (params (Key :type "Key Structure"))
  (bind _playerref (`self.PlayerRef`))
  (bind _playerref_2 (`self.PlayerRef`))
  (bind _playerref_3 (`self.PlayerRef`))
  (bind _playerref_4 (`self.PlayerRef`))
  (bind _dialogonpcref (`/Game/ThirdPerson/Blueprints/BP_ThirdPersonCharacter.DialogoNPCRef` (`self.PlayerRef`)))
  (bind _dialogonpcref_2 (`/Game/ThirdPerson/Blueprints/BP_ThirdPersonCharacter.DialogoNPCRef` (`self.PlayerRef`)))
  ; interagir com o NPC (E)
  (:`Pressed`
    (`/Engine/EditorBlueprintResources/StandardMacros.IsValid` _playerref_3
      (:`Is Valid`
        (if (`/Game/ThirdPerson/Blueprints/BP_ThirdPersonCharacter.QuestVespasConcluida` _playerref_3)
          (if (`/Game/ThirdPerson/Blueprints/BP_ThirdPersonCharacter.EfeitoQuestVespaJaTocou` (`self.PlayerRef`))
            (switch `int` (`KismetMathLibrary.Conv_Int64ToInt` (`self.FinalQuestIndex`))
              (:`0`
                (`/Game/Programação_Geral/Missoes/WB_Dialogo_NPC.MostrarDialogoNPC` _dialogonpcref "Graças a você, a estrada para a mina voltou a ser segura. Fazia muito tempo que eu não via esperança nos olhos desse povo.")
                (set `self.FinalQuestIndex` 1))
              (:`1`
                (`/Game/Programação_Geral/Missoes/WB_Dialogo_NPC.MostrarDialogoNPC` _dialogonpcref "Caso esteja procurando um novo desafio, vi que o alquimista que se mudou para o topo do morro está precisando de ajuda.")
                (set `self.FinalQuestIndex` 2))
              (:`2`
                (`/Game/Programação_Geral/Missoes/WB_Dialogo_NPC.EsconderDialogoNPC` _dialogonpcref)
                (`/Game/Programação_Geral/Missoes/Wb_Quest.EsconderMissãoVespa` (`/Game/ThirdPerson/Blueprints/BP_ThirdPersonCharacter.QuestHUDRef` (`self.PlayerRef`)))
                (if (not (`/Game/ThirdPerson/Blueprints/BP_ThirdPersonCharacter.EfeitoTransiçãoJáPassou` _playerref_2))
                  (`Widget.SetVisibility` (`/Game/ThirdPerson/Blueprints/BP_ThirdPersonCharacter.TransicaoQuestRef` _playerref_2) "Visible")
                  (`KismetSystemLibrary.Delay` 0.5)
                  (for _array_element (`self.EstruturasParaAparecer`)
                    (`self.SetActorHiddenInGame` _array_element false)
                    (`self.SetActorEnableCollision` _array_element true)
                    (`KismetSystemLibrary.Delay` 0.5)
                    (`Widget.SetVisibility` (`/Game/ThirdPerson/Blueprints/BP_ThirdPersonCharacter.TransicaoQuestRef` _playerref_4) "Hidden")
                    (set `/Game/ThirdPerson/Blueprints/BP_ThirdPersonCharacter.EfeitoTransiçãoJáPassou` true _playerref_4)))))
            (else
              (`ActorComponent.SetActive` (`self.Niagara`) true true)
              (`KismetSystemLibrary.Delay` 1.0)
              (set `/Game/ThirdPerson/Blueprints/BP_ThirdPersonCharacter.EfeitoQuestVespaJaTocou` true (`self.PlayerRef`))))
          (elif (`/Game/ThirdPerson/Blueprints/BP_ThirdPersonCharacter.QuestVespasAceita` _playerref_3)
            (if (>= (`/Game/ThirdPerson/Blueprints/BP_ThirdPersonCharacter.VespasMortas` (`self.PlayerRef`)) 3)
              (set `/Game/ThirdPerson/Blueprints/BP_ThirdPersonCharacter.QuestVespasConcluida` true (`self.PlayerRef`)))
            (else
              (switch `int` (`KismetMathLibrary.Conv_Int64ToInt` (`self.IntroQuestIndex`))
                (:`0`
                  (`/Game/Programação_Geral/Missoes/WB_Dialogo_NPC.MostrarDialogoNPC` _dialogonpcref_2 "Ah... um visitante. Faz tempo que não vejo alguém passar por estas estradas.")
                  (set `self.IntroQuestIndex` 1))
                (:`1`
                  (`/Game/Programação_Geral/Missoes/WB_Dialogo_NPC.MostrarDialogoNPC` _dialogonpcref_2 "Nossa vila fica distante de tudo. Nunca tivemos muitos visitantes, fico surpreso de ver você por aqui.")
                  (set `self.IntroQuestIndex` 2))
                (:`2`
                  (`/Game/Programação_Geral/Missoes/WB_Dialogo_NPC.MostrarDialogoNPC` _dialogonpcref_2 "Nossa vila era até que prospera, porém tudo piorou quando criaturas começaram a aparecer nas redondezas. Aos poucos, a vila foi ficando esquecida.")
                  (set `self.IntroQuestIndex` 3))
                (:`3`
                  (`/Game/Programação_Geral/Missoes/WB_Dialogo_NPC.MostrarDialogoNPC` _dialogonpcref_2 "O maior problema está na estrada que leva até a mina. Vespas venenosas fizeram ninho por lá e agora não consigo os materiais para construir as casas.")
                  (set `self.IntroQuestIndex` 4))
                (:`4`
                  (`/Game/Programação_Geral/Missoes/WB_Dialogo_NPC.MostrarDialogoNPC` _dialogonpcref_2 "Sem essa estrada, ninguém consegue chegar aos minérios e principalmente aos cristais. E sem eles não temos como manter a vila viva.")
                  (set `self.IntroQuestIndex` 5))
                (:`5`
                  (`/Game/Programação_Geral/Missoes/WB_Dialogo_NPC.MostrarDialogoNPC` _dialogonpcref_2 "Você poderia nos ajudar? Elimine as vespas venenosas na estrada da mina e volte para falar comigo.")
                  (set `self.IntroQuestIndex` 6))
                (:`6`
                  (`/Game/Programação_Geral/Missoes/WB_Dialogo_NPC.EsconderDialogoNPC` _dialogonpcref_2)
                  (set `/Game/ThirdPerson/Blueprints/BP_ThirdPersonCharacter.QuestVespasAceita` true _playerref)
                  (set `/Game/ThirdPerson/Blueprints/BP_ThirdPersonCharacter.VespasMortas` 0 _playerref)
                  (`/Game/Programação_Geral/Missoes/Wb_Quest.MostrarQuestVespas` (`/Game/ThirdPerson/Blueprints/BP_ThirdPersonCharacter.QuestHUDRef` _playerref)))))))))))

(fn `UserConstructionScript`)