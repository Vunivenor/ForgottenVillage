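; BP_Arma_2 is a metal sword weapon actor that registers when the third-person character touches it.
; On overlap with the EspadaDeMetal component, it casts the other actor to BP_ThirdPersonCharacter and sets that character's PegouAEspada (picked up sword) flag.
; It then makes its own sword component visible in game, without attaching or destroying it.
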(event `self.EspadaDeMetal.OnComponentBeginOverlap`
  (params (OverlappedComponent :type "PrimitiveComponent Object Reference") (OtherActor :type "Actor Object Reference") (OtherComp :type "PrimitiveComponent Object Reference") (OtherBodyIndex :type Integer) (bFromSweep :type Boolean) (SweepResult :type "HitResult Structure (by ref)"))
  (bind _asbp_third_person_character (cast `/Game/ThirdPerson/Blueprints/BP_ThirdPersonCharacter` OtherActor))
  (set `/Game/ThirdPerson/Blueprints/BP_ThirdPersonCharacter.Pegou a Espada` true _asbp_third_person_character)
  (`SceneComponent.SetHiddenInGame` (`self.EspadaDeMetal`) false false))

(fn `UserConstructionScript`
  (`parent.UserConstructionScript`))