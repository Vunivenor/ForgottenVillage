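; Bear enemy that wanders to random reachable points, chases pawns it sees via PawnSensing and plays a random attack montage on arrival.
; Movement uses recursive AIMoveTo calls, locked during attacks.
; Tick shows a player-facing health bar when the player is nearby.
; AnyDamage plays hit reactions and reduces health; death plays a montage, updates the player's bear quest count and HUD if active, then destroys the actor.
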(event `Andar Pelo Mapa`
  ;[1 1 1] Andar pelo mapa de modo aleatorio
  (`|AIMoveTo` self (`NavigationSystemV1.K2_GetRandomReachablePointInRadius` (`self.K2_GetActorLocation`) 3000.0 null null) null
    (:`then`
      (`GameplayStatics.PlaySound2D` "/Game/Criaturas/Urso/Audio/UrsoRespiração.UrsoRespiração" 1.0 1.0 0.0 null null))
    (:`OnSuccess`
      (`KismetSystemLibrary.Delay` 3.0 :!label _label)
      (`self.Andar Pelo Mapa`))
    (:`OnFail`
      (goto _label))))

(event `self.ReceiveBeginPlay`
  ;[1 1 1] Andar pelo mapa de modo aleatorio
  (`self.Andar Pelo Mapa`))

(event `self.PawnSensing.OnSeePawn`
  (params (Pawn :type "Pawn Object Reference"))
  ;[1 1 1] Seguir o Player que ver
  (`|AIMoveTo` self (0.0 0.0 0.0) Pawn 10.0
    (:`OnSuccess`
      ;[1 1 1] Bater quando chegar perto
      (if (`self.Pode Levar Dano?`)
        (`CharacterMovementComponent.DisableMovement` (`self.CharacterMovement`))
        (`|PlayMontage` (`self.Mesh`) (`KismetArrayLibrary.Array_Random` (`self.Montage Ataque Urso`)) 1.0 0.0 "None" false
          (:`then`
            (`GameplayStatics.PlaySound2D` "/Game/Criaturas/Urso/Audio/UrsoRugido__3_.UrsoRugido__3_" 1.0 1.0 0.0 null null))
          (:`OnCompleted`
            (`CharacterMovementComponent.SetMovementMode` (`self.CharacterMovement`) "MOVE_Walking" 0 :!label _label_2)
            (`KismetSystemLibrary.Delay` 0.2)
            (`self.Andar Pelo Mapa`))
          (:`OnInterrupted`
            (goto _label_2)))))))

(event `self.ReceiveTick`
  (params (DeltaSeconds :type "Float (single-precision)"))
  (bind _barra_de_vida_urso (`self.Barra de Vida Urso`))
  (bind _barra_de_vida_urso_2 (`self.Barra de Vida Urso`))
  ;[1 1 1] Barra de vida do inimigo
  (if (< (`KismetMathLibrary.VSize` (- (`self.K2_GetActorLocation` (`GameplayStatics.GetPlayerCharacter` 0)) (`self.K2_GetActorLocation`))) 2000.0)
    (`SceneComponent.SetVisibility` _barra_de_vida_urso true false)
    (`SceneComponent.K2_SetWorldRotation` _barra_de_vida_urso_2 (`KismetMathLibrary.FindLookAtRotation` (`self.K2_GetActorLocation`) (`self.K2_GetActorLocation` (`GameplayStatics.GetPlayerCharacter` 0))) false false)
    (bind _aswb_barra_de_vida_inimigo_urso (cast `/Game/Criaturas/Urso/Blueprints/WB_Barra_de_Vida_Inimigo_Urso` (`WidgetComponent.GetWidget` _barra_de_vida_urso_2)))
    (`ProgressBar.SetPercent` (`/Game/Criaturas/Urso/Blueprints/WB_Barra_de_Vida_Inimigo_Urso.Barradevidadoinimigourso` _aswb_barra_de_vida_inimigo_urso) (/ (`self.Vida Atual`) 200.0))
    (else
      (`SceneComponent.SetVisibility` _barra_de_vida_urso false false))))

(event `self.ReceiveAnyDamage`
  (params (Damage :type "Float (single-precision)") (DamageType :type "DamageType Object Reference") (InstigatedBy :type "Controller Object Reference") (DamageCauser :type "Actor Object Reference"))
  (bind _vida_atual (`self.Vida Atual`))
  ;[1 1 1] Inimigo leva dano e efetua a animação de dano, além de morrer se a barra de vida for menor ou igual a 0
  (set `self.Pode Levar Dano?` false)
  (if (not (<= _vida_atual 0.0))
    (`|PlayMontage` (`self.Mesh`) (`KismetArrayLibrary.Array_Random` (`self.Montage Dano`)) 1.7
      (:`then`
        (bind _output_get (set `self.Vida Atual` (- _vida_atual Damage)))
        (`GameplayStatics.PlaySound2D` "/Game/Criaturas/Urso/Audio/UrsoRugido.UrsoRugido" 1.0 1.0 0.0 null null))
      (:`OnCompleted`
        (if (> _output_get 1.0) :!label _label_3
          (set `self.Pode Levar Dano?` true)
          (else
            (`CharacterMovementComponent.DisableMovement` (`self.CharacterMovement`))
            (`|PlayMontage` (`self.Mesh`) "/Game/Criaturas/Urso/Animações/ANM_Urso_Morte.ANM_Urso_Morte" 0.5
              (:`then`
                (bind _asbp_third_person_character (cast `/Game/ThirdPerson/Blueprints/BP_ThirdPersonCharacter` (`GameplayStatics.GetPlayerCharacter` 0)))
                (if (`/Game/ThirdPerson/Blueprints/BP_ThirdPersonCharacter.QuestUrsoAceita` _asbp_third_person_character)
                  (if (not (`/Game/ThirdPerson/Blueprints/BP_ThirdPersonCharacter.QuestUrsoConcluida` _asbp_third_person_character))
                    (set `/Game/ThirdPerson/Blueprints/BP_ThirdPersonCharacter.UrsoMorto` (+ (`/Game/ThirdPerson/Blueprints/BP_ThirdPersonCharacter.UrsoMorto` _asbp_third_person_character) 1) _asbp_third_person_character)
                    (`/Game/Programação_Geral/Missoes/Wb_Quest.AtualizarProgressoUrso` (`/Game/ThirdPerson/Blueprints/BP_ThirdPersonCharacter.QuestHUDRef` _asbp_third_person_character) (`/Game/ThirdPerson/Blueprints/BP_ThirdPersonCharacter.UrsoMorto` _asbp_third_person_character)))))
              (:`OnCompleted`
                (`self.K2_DestroyActor`))))))
      (:`OnInterrupted`
        (goto _label_3)))))

(fn `Bear dead`)

(fn `UserConstructionScript`)