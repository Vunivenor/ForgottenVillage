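; BP_NPC_Test_Quest is a test quest-giver NPC for a wasp quest ("QuestVespas").
; A sphere overlap stores the player, enables input and prints a talk prompt, and leaving it clears both the reference and the input.
; Pressing E accepts the quest on the player character, resets the wasp kill count and shows the quest HUD.
; If the quest is already completed, E turns off the NPC's Niagara effect instead.
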(event `self.Sphere.OnComponentBeginOverlap`
  (params (OverlappedComponent :type "PrimitiveComponent Object Reference") (OtherActor :type "Actor Object Reference") (OtherComp :type "PrimitiveComponent Object Reference") (OtherBodyIndex :type Integer) (bFromSweep :type Boolean) (SweepResult :type "HitResult Structure (by ref)"))
  ; Colidir com o NPC para aparecer a Interação
  (bind _asbp_third_person_character (cast `/Game/ThirdPerson/Blueprints/BP_ThirdPersonCharacter` OtherActor))
  (set `self.PlayerRef` _asbp_third_person_character)
  (`self.EnableInput` (`GameplayStatics.GetPlayerController` 0))
  (`KismetSystemLibrary.PrintString` "Pressione \"E\" para conversar"))

(event `self.Sphere.OnComponentEndOverlap`
  (params (OverlappedComponent :type "PrimitiveComponent Object Reference") (OtherActor :type "Actor Object Reference") (OtherComp :type "PrimitiveComponent Object Reference") (OtherBodyIndex :type Integer))
  ; Colidir com o NPC para aparecer a Interação
  (cast `/Game/ThirdPerson/Blueprints/BP_ThirdPersonCharacter` OtherActor)
  (set `self.PlayerRef` null)
  (`self.DisableInput` (`GameplayStatics.GetPlayerController` 0)))

(event `Key|E`
  (params (Key :type "Key Structure"))
  (bind _playerref (`self.PlayerRef`))
  (bind _playerref_2 (`self.PlayerRef`))
  ; interagir com o NPC (E)
  (:`Pressed`
    (`/Engine/EditorBlueprintResources/StandardMacros.IsValid` _playerref
      (:`Is Valid`
        (if (`/Game/ThirdPerson/Blueprints/BP_ThirdPersonCharacter.QuestVespasConcluida` _playerref)
          (`ActorComponent.SetActive` (`self.Niagara`) false false)
          (elif (not (`/Game/ThirdPerson/Blueprints/BP_ThirdPersonCharacter.QuestVespasAceita` _playerref))
            (set `/Game/ThirdPerson/Blueprints/BP_ThirdPersonCharacter.QuestVespasAceita` true _playerref_2)
            (set `/Game/ThirdPerson/Blueprints/BP_ThirdPersonCharacter.VespasMortas` 0 _playerref_2)
            (`/Game/Programação_Geral/Missoes/MissõesSimon/WB_Quest_Vespa.MostrarQuestVespas` (`/Game/ThirdPerson/Blueprints/BP_ThirdPersonCharacter.VariavelQuestVespaHUD` _playerref_2))))))))

(fn `UserConstructionScript`)