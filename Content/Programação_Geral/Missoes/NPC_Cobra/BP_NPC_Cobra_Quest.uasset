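; Quest-giver NPC, an alchemist who sends the player to kill an ancient snake for its scales.
; Sphere overlap shows an interaction text, enables E input and sets the player's ColidindoQuestVespa flag.
; E steps through indexed intro and completion dialogues, with quest state and widget references kept on BP_ThirdPersonCharacter.
; Completion fires a one-time Niagara effect, then, after the dialogue, reveals structures hidden since BeginPlay behind a transition widget.
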(event `self.ReceiveBeginPlay`
  ; Estruturas começam invisivéis no começo do jogo
  (for _array_element (`self.EstruturasParaAparecerCobra`)
    (`self.SetActorHiddenInGame` _array_element true)
    (`self.SetActorEnableCollision` _array_element false)))

(event `self.Sphere.OnComponentBeginOverlap`
  (params (OverlappedComponent :type "PrimitiveComponent Object Reference") (OtherActor :type "Actor Object Reference") (OtherComp :type "PrimitiveComponent Object Reference") (OtherBodyIndex :type Integer) (bFromSweep :type Boolean) (SweepResult :type "HitResult Structure (by ref)"))
  ; Colidir com o NPC para aparecer a Interação
  (bind _asbp_third_person_character (cast `/Game/ThirdPerson/Blueprints/BP_ThirdPersonCharacter` OtherActor))
  (bind _output_get (set `self.PlayerRef` _asbp_third_person_character))
  (`self.EnableInput` (`GameplayStatics.GetPlayerController` 0))
  (set `/Game/ThirdPerson/Blueprints/BP_ThirdPersonCharacter.ColidindoQuestVespa?` true _output_get)
  (`SceneComponent.SetHiddenInGame` (`self.Texto`) false false)
  (`SceneComponent.K2_SetWorldRotation` (`self.Texto`) (`KismetMathLibrary.FindLookAtRotation` (`self.K2_GetActorLocation`) (`self.K2_GetActorLocation` (`GameplayStatics.GetPlayerCharacter` 0))) false false))

(event `self.Sphere.OnComponentEndOverlap`
  (params (OverlappedComponent :type "PrimitiveComponent Object Reference") (OtherActor :type "Actor Object Reference") (OtherComp :type "PrimitiveComponent Object Reference") (OtherBodyIndex :type Integer))
  ; Colidir com o NPC para aparecer a Interação
  (bind _asbp_third_person_character (cast `/Game/ThirdPerson/Blueprints/BP_ThirdPersonCharacter` OtherActor))
  (bind _output_get (set `self.PlayerRef` _asbp_third_person_character))
  (`self.DisableInput` (`GameplayStatics.GetPlayerController` 0))
  (set `/Game/ThirdPerson/Blueprints/BP_ThirdPersonCharacter.ColidindoQuestVespa?` false _output_get)
  (`SceneComponent.SetHiddenInGame` (`self.Texto`) true false)
  (`self.DisableInput` (`GameplayStatics.GetPlayerController` 0)))

(event `Key|E`
  (params (Key :type "Key Structure"))
  (bind _playerref (`self.PlayerRef`))
  (bind _playerref_2 (`self.PlayerRef`))
  (bind _playerref_3 (`self.PlayerRef`))
  (bind _dialogonpccobraref (`/Game/ThirdPerson/Blueprints/BP_ThirdPersonCharacter.DialogoNpcCobraRef` (`self.PlayerRef`)))
  (bind _dialogonpccobraref_2 (`/Game/ThirdPerson/Blueprints/BP_ThirdPersonCharacter.DialogoNpcCobraRef` _playerref_2))
  ; interagir com o NPC (E)
  (:`Pressed`
    (`/Engine/EditorBlueprintResources/StandardMacros.IsValid` _playerref_3
      (:`Is Valid`
        (if (`/Game/ThirdPerson/Blueprints/BP_ThirdPersonCharacter.QuestCobraConcluida` _playerref_3)
          (if (`/Game/ThirdPerson/Blueprints/BP_ThirdPersonCharacter.EfeitoQuestCobraJaTocou` (`self.PlayerRef`))
            (switch `int` (`KismetMathLibrary.Conv_Int64ToInt` (`self.FinalQuestIndex`))
              (:`0`
                (`/Game/Programação_Geral/Missoes/NPC_Cobra/WB_Dialogo_NPC_Cobra.MostrarDialogoNPC` _dialogonpccobraref_2 "Você conseguiu as escamas... excelente. Com elas, meus experimentos poderão avançar muito além do que eu esperava.")
                (set `self.FinalQuestIndex` 1))
              (:`1`
                (`/Game/Programação_Geral/Missoes/NPC_Cobra/WB_Dialogo_NPC_Cobra.MostrarDialogoNPC` _dialogonpccobraref_2 "Quanto à sua recompensa, vi algo que parece de seu agrado em uma antiga ruína próxima daqui. E se ainda tiver disposição, procure o senhor do moinho... ele também precisa de ajuda.")
                (set `self.FinalQuestIndex` 2))
              (:`2`
                (`/Game/Programação_Geral/Missoes/NPC_Cobra/WB_Dialogo_NPC_Cobra.EsconderDialogoNPC` _dialogonpccobraref_2)
                (`/Game/Programação_Geral/Missoes/NPC_Cobra/WB_Quest_Cobra.EsconderMissãoCobra` (`/Game/ThirdPerson/Blueprints/BP_ThirdPersonCharacter.QuestCobraHudRef` _playerref_2))
                (`Widget.SetVisibility` (`/Game/ThirdPerson/Blueprints/BP_ThirdPersonCharacter.TransicaoQuestRef` (`self.PlayerRef`)) "Visible")
                (`KismetSystemLibrary.Delay` 0.5)
                (for _array_element (`self.EstruturasParaAparecerCobra`)
                  (`self.SetActorHiddenInGame` _array_element false)
                  (`self.SetActorEnableCollision` _array_element true)
                  (`KismetSystemLibrary.Delay` 0.5)
                  (`Widget.SetVisibility` (`/Game/ThirdPerson/Blueprints/BP_ThirdPersonCharacter.TransicaoQuestRef` (`self.PlayerRef`)) "Hidden"))))
            (else
              (`ActorComponent.SetActive` (`self.Niagara`) true true)
              (`KismetSystemLibrary.Delay` 1.0)
              (set `/Game/ThirdPerson/Blueprints/BP_ThirdPersonCharacter.EfeitoQuestCobraJaTocou` true (`self.PlayerRef`))))
          (elif (`/Game/ThirdPerson/Blueprints/BP_ThirdPersonCharacter.QuestCobraAceita` _playerref_3)
            (if (>= (`/Game/ThirdPerson/Blueprints/BP_ThirdPersonCharacter.CobraMorta` (`self.PlayerRef`)) 1)
              (set `/Game/ThirdPerson/Blueprints/BP_ThirdPersonCharacter.QuestCobraConcluida` true (`self.PlayerRef`)))
            (else
              (switch `int` (`KismetMathLibrary.Conv_Int64ToInt` (`self.IntroQuestIndex`))
                (:`0`
                  (`/Game/Programação_Geral/Missoes/NPC_Cobra/WB_Dialogo_NPC_Cobra.MostrarDialogoNPC` _dialogonpccobraref "Ah, viajante... aproxime-se. Poucos chegam até minha pequena casa sem se assustar com os sons e fumaças daqui.")
                  (set `self.IntroQuestIndex` 1))
                (:`1`
                  (`/Game/Programação_Geral/Missoes/NPC_Cobra/WB_Dialogo_NPC_Cobra.MostrarDialogoNPC` _dialogonpccobraref "Sou alquimista, e meus estudos precisam de materiais raros. As escamas de uma cobra antiga possuem propriedades que podem fortalecer minhas poções.")
                  (set `self.IntroQuestIndex` 2))
                (:`2`
                  (`/Game/Programação_Geral/Missoes/NPC_Cobra/WB_Dialogo_NPC_Cobra.MostrarDialogoNPC` _dialogonpccobraref "Essa cobra vive perto das pedras antigas, além da trilha. Não é uma criatura comum, então tome cuidado ao enfrentá-la.")
                  (set `self.IntroQuestIndex` 3))
                (:`3`
                  (`/Game/Programação_Geral/Missoes/NPC_Cobra/WB_Dialogo_NPC_Cobra.MostrarDialogoNPC` _dialogonpccobraref "Traga-me algumas escamas dela, e eu poderei continuar meus experimentos. Se fizer isso, terei uma recompensa para você.")
                  (set `self.IntroQuestIndex` 4))
                (:`4`
                  (`/Game/Programação_Geral/Missoes/NPC_Cobra/WB_Dialogo_NPC_Cobra.EsconderDialogoNPC` _dialogonpccobraref)
                  (set `/Game/ThirdPerson/Blueprints/BP_ThirdPersonCharacter.QuestCobraAceita` true _playerref)
                  (set `/Game/ThirdPerson/Blueprints/BP_ThirdPersonCharacter.CobraMorta` 0 _playerref)
                  (`/Game/Programação_Geral/Missoes/NPC_Cobra/WB_Quest_Cobra.MostrarQuestCobra` (`/Game/ThirdPerson/Blueprints/BP_ThirdPersonCharacter.QuestCobraHudRef` _playerref)))))))))))

(fn `UserConstructionScript`)